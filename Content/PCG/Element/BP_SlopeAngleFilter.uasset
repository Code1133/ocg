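; Custom PCG element "Slope Angle Filter" that keeps only points whose slope angle lies between MinAngle and MaxAngle.
; It derives each angle as the arccosine of point density in degrees, so it treats incoming density as the cosine of the slope.
; Each input on "In" yields point data on "Out", filled from a FilteredPoints array that is not cleared between inputs.
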(fn ExecutewithContext
  (params (InContext :type PCG%20Context%20Structure%20%28by%20ref%29) (Input :type PCG%20Data%20Collection%20Structure%20%28by%20ref%29))
  (bind _returnvalue (Data|GetTypedInputsbyPinLabel Input "In" "/Script/PCG.PCGPointData"))
  (for _array_element _returnvalue
    (bind _output_get (LocalVariables|SetCurrentPointData _array_element))
    (for _array_element_2 (SpatialData|GetPoints _output_get)
      (bind _output_get_2 (LocalVariables|SetCurrentPoint _array_element_2))
      (if (Math|Float|InRange(Float) (Math|Trig|RadiansToDegrees (Math|Trig|Acos(Degrees) (.Density (Utilities|Struct|BreakPCGPoint _output_get_2)))) (Variables|Default|GetMinAngle) (Variables|Default|GetMaxAngle))
        (Utilities|Array|Add (LocalVariables|GetFilteredPoints) (LocalVariables|GetCurrentPoint))))
    ;[0.15 0.15 0.15 0.5] Construct Output Point Data
    (bind _returnvalue_2 (Game|ConstructObjectfromClass "/Script/PCG.PCGPointData"))
    (bind _output_get_3 (LocalVariables|SetOutPointData _returnvalue_2))
    (SpatialData|InitializefromData _output_get_3 (LocalVariables|GetCurrentPointData) 0 true true)
    ;[0.15 0.15 0.15 0.5] Set Points
    (SpatialData|SetPoints (LocalVariables|GetOutPointData) (LocalVariables|GetFilteredPoints))
    ;[0.15 0.15 0.15 0.5] Construct Data Collection
    (Class|PCGDataFunctionLibrary|AddtoCollection (LocalVariables|GetOutputDataCollection) (LocalVariables|GetOutPointData) "Out" (Utilities|Array|MakeArray)))
  (return (LocalVariables|GetOutputDataCollection)))

(fn NodeTitleOverride
  (return (Utilities|Name|MakeLiteralName "Slope Angle Filter")))